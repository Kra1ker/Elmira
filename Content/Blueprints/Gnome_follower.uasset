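; Gnome follower pawn that chases the third-person character and catches it.
; While awake it issues an AI MoveTo toward the player every Tick.
; On reaching the player it stops moving, calls GotCaught, plays a cackle and swaps the gnome material.
; A DoOnce keeps the catch single-shot while it sleeps for a delay, then it restores material and movement and resumes the chase.
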(event `self.ReceiveBeginPlay`
  (bind _returnvalue (`GameplayStatics.GetActorOfClass` "/Game/ThirdPerson/Blueprints/BP_ThirdPersonCharacter.BP_ThirdPersonCharacter_C"))
  (set `self.TP_Character` _returnvalue)
  (`SceneComponent.K2_SetRelativeRotation` (`self.GnomeSM`) (struct :`Yaw` -90.0) false false))

(event `self.ReceiveTick`
  (params (DeltaSeconds :type "Float (single-precision)"))
  (bind _tp_character (`self.TP_Character`))
  (bind _charactermovement (`self.CharacterMovement`))
  (bind _returnvalue_location (`KismetMathLibrary.BreakTransform` (`self.GetTransform` self)))
  (if (!= (`self.isSleep`) true)
    (`|AIMoveTo` self (0.0 0.0 0.0) _tp_character 50.0
      (:`OnSuccess`
        (`ActorComponent.Deactivate` _charactermovement)
        (`/Engine/EditorBlueprintResources/StandardMacros.DoOnce` false :!label _label
          (:`Completed`
            (`/Game/ThirdPerson/Blueprints/BP_ThirdPersonCharacter.GotCaught` _tp_character)
            (`GameplayStatics.PlaySoundAtLocation` "/Game/Characters/Gnome/alien-cackle-99968.alien-cackle-99968" _returnvalue_location (struct) 1.0 1.0 0.0 null null null null)
            (`PrimitiveComponent.SetMaterial` (`self.GnomeSM`) 0 "/Game/Characters/Gnome/garden_gnome_02.garden_gnome_02")
            (set `self.isSleep` true)
            (`KismetSystemLibrary.Delay` 10.0)
            (`PrimitiveComponent.SetMaterial` (`self.GnomeSM`) 0 "/Game/Characters/Gnome/garden_gnome_01.garden_gnome_01")
            (set `self.isSleep` false)
            (`ActorComponent.Activate` _charactermovement false)
            (goto _label :!via `Reset`)))))))

(fn `UserConstructionScript`)